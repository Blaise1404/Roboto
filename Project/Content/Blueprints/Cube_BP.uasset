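; Clickable cube actor with configurable colour that reports clicks to the VR player controller.
; On click, it casts the first player controller to VR_PlayerController and passes itself to CubeClicked.
; The construction script builds a dynamic material instance from the Material variable on the static mesh, applying the Colour and DiffStrengh variables as shader parameters.
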(event EventBeginPlay)

(event Collision|EventActorBeginOverlap
  (params (OtherActor :type Actor%20Object%20Reference)))

(event EventTick
  (params (DeltaSeconds :type Float%20%28single-precision%29)))

(event MouseInput|EventActorOnClicked
  (params (ButtonPressed :type Key%20Structure))
  (bind _asvr_player_controller (Utilities|Casting|CastToVR_PlayerController (Game|GetPlayerController 0)))
  (Default|CubeClicked _asvr_player_controller self))

(fn ConstructionScript
  (bind _staticmesh (Variables|Default|GetStaticMesh))
  (bind _returnvalue (Rendering|Material|CreateDynamicMaterialInstance _staticmesh 0 (Variables|Default|GetMaterial) "None" :!class /Script/Engine.PrimitiveComponent))
  (Rendering|Material|SetMaterial _staticmesh 0 _returnvalue)
  (Rendering|Material|SetVectorParameterValue _returnvalue "Color1" (Variables|Default|GetColour) :!class /Script/Engine.MaterialInstanceDynamic)
  (Rendering|Material|SetScalarParameterValue _returnvalue "Diff" (Variables|Default|GetDiffStrengh) :!class /Script/Engine.MaterialInstanceDynamic))